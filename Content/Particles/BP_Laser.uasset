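; BP_Laser is a laser actor in the particles folder that animates the color of its Sphere component.
; The construction script creates a dynamic material instance on the sphere and stores it.
; On BeginPlay, a timeline starts and writes its track value into that material's Color parameter on every update.
; Disconnected color-toggle logic comparing stored colors remains in the construction script but never runs.
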(event EventBeginPlay
  (bind _newtrack_1 (Timeline|Timeline_0 PlayFromStart)
    (:Update
      (Rendering|Material|SetVectorParameterValue (Variables|Default|GetDynamMaterial) "Color" _newtrack_1 :!class /Script/Engine.MaterialInstanceDynamic))))

(event Collision|EventActorBeginOverlap
  (params (OtherActor :type Actor%20Object%20Reference)))

(event EventTick
  (params (DeltaSeconds :type Float%20%28single-precision%29)))

(fn ConstructionScript
  (bind _returnvalue (Rendering|Material|CreateDynamicMaterialInstance (Variables|Default|GetSphere) 0 "/Game/Particles/Particule_Textures/Mat_Dynam_Inst.Mat_Dynam_Inst" :!class /Script/Engine.PrimitiveComponent))
  (Variables|Default|SetDynamMaterial _returnvalue))