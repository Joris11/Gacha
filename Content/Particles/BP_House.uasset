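; BP_House is a two-floor house actor that varies its look through random floor orientation.
; The construction script independently adds a random local yaw of 0, 90 or 180 degrees to the FirstFloor and SecondFloor components.
; A random pick from RoofArray and a Roof reference are present but unconnected, and the event graph has no active logic.
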(event EventBeginPlay)

(event Collision|EventActorBeginOverlap
  (params (OtherActor :type Actor%20Object%20Reference)))

(event EventTick
  (params (DeltaSeconds :type Float%20%28single-precision%29)))

(fn ConstructionScript
  (Transformation|AddLocalRotation (Variables|Default|GetFirst%20Floor) (Math|Rotator|MakeRotator 0.0 0.0 (* (Math|Random|RandomInteger 3) 9e+01)) false false)
  (Transformation|AddLocalRotation (Variables|Default|GetSecond%20Floor) (Math|Rotator|MakeRotator 0.0 0.0 (* (Math|Random|RandomInteger 3) 9e+01)) false false))