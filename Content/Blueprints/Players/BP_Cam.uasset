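; BP_Cam is a player camera actor whose follow logic is currently disconnected, so it does not move the camera.
; Live events only store StopInterpX/StopInterpY from interface calls and set IsStoppedBOOP when an actor named "Freddy" ends overlap.
; Unwired leftovers show the intended technique: VInterpTo the camera toward the player's capsule in X/Y, freezing either axis by flag.
; Tick, BeginPlay and the construction script are empty.
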(event EventBeginPlay)

(event Collision|EventActorEndOverlap
  (params (OtherActor :type Actor%20Object%20Reference))
  (if (Utilities|Enum|Equal(Enum) (Utilities|GetDisplayName OtherActor) "Freddy")
    (Variables|Default|SetisStoppedBOOP true)))

(event EventTick
  (params (DeltaSeconds :type Float%20%28single-precision%29)))

(event Collision|EventActorBeginOverlap
  (params (OtherActor :type Actor%20Object%20Reference)))

(event EventInterfaceStopInterpX
  (params (StopInterpX :type Boolean))
  (Variables|Default|SetStopInterpX StopInterpX))

(event EventInterfaceStopInterpY
  (params (StopInterpY :type Boolean))
  (Variables|Default|SetStopInterpY StopInterpY))

(fn ConstructionScript)