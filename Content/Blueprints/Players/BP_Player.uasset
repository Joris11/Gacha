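; Player pawn that moves along its mesh's axes and builds elemental towers at spawn points.
; Overlapping a free BP_TowerSpawnPoint enables building and stores its location.
; Air, Earth, Fire and Water inputs fill a two-slot combination, which InputToTower maps to a tower type, spawning and initializing a cone, sphere or base tower.
; The construction script also fills a DicTowers map, but lookup uses InputToTower's nested switches instead.
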(event OnComponentBeginOverlap(InteractTrigger)
  (params (OverlappedComponent :type Primitive%20Component%20Object%20Reference) (OtherActor :type Actor%20Object%20Reference) (OtherComp :type Primitive%20Component%20Object%20Reference) (OtherBodyIndex :type Integer) (bFromSweep :type Boolean) (SweepResult :type Hit%20Result%20Structure%20%28by%20ref%29))
  ;[1 1 1] Allows / Disallows tower creation
  (bind _asbp_tower_spawn_point (Utilities|Casting|CastToBP_TowerSpawnPoint OtherActor))
  (Variables|Default|SetCanBuild (Variables|/Game/Blueprints/Actors/GameplayElement/BP_TowerSpawnPoint.BP_TowerSpawnPoint_C|GetM%20IsFreeSlot _asbp_tower_spawn_point))
  (Variables|Default|SetTowerPoint (Transformation|GetActorLocation _asbp_tower_spawn_point))
  (Development|PrintString "ABLE TO CREATE"))

(event OnComponentEndOverlap(InteractTrigger)
  (params (OverlappedComponent :type Primitive%20Component%20Object%20Reference) (OtherActor :type Actor%20Object%20Reference) (OtherComp :type Primitive%20Component%20Object%20Reference) (OtherBodyIndex :type Integer))
  ;[1 1 1] Allows / Disallows tower creation
  (Utilities|Casting|CastToBP_TowerSpawnPoint OtherActor)
  (Variables|Default|SetCanBuild false)
  (Variables|Default|SetTowerPoint "0, 0, 0"))

(event EventBeginPlay)

(event Collision|EventActorBeginOverlap
  (params (OtherActor :type Actor%20Object%20Reference)))

(event EventTick
  (params (DeltaSeconds :type Float%20%28single-precision%29)))

(event Input|ActionEvents|InputActionElem_Air
  (params (Key :type Key%20Structure))
  (bind _towerpoint (Variables|Default|GetTowerPoint))
  ;[1 1 1] Input combinations
  (:Pressed
    (if (Variables|Default|GetCanBuild)
      (if (Utilities|Enum|Equal(Enum) (.elem1 (Variables|Default|GetInputCombination)) "NewEnumerator0")
        (Variables|Default|SetInputCombination (Utilities|Struct|MakeSTRUCT_ElemToTowers (.elem1 (Variables|Default|GetInputCombination)) "NewEnumerator2"))
        (bind _towertype (CallFunction|InputtoTower (Variables|Default|GetInputCombination)))
        (switch Utilities|FlowControl|Switch|SwitchonENUM_Towers _towertype
          (:NewEnumerator0
            ;[1 1 1] Cone tower
            (bind _returnvalue (Game|SpawnActorfromClass "/Game/Blueprints/Actors/Towers/Parents/BP_ConeTower.BP_ConeTower_C" (Math|Transform|MakeTransform _towerpoint "0, 0, 0" "1,1,1") "Undefined" 0 0))
            (Default|Init _returnvalue _towertype))
          (:NewEnumerator1
            ;[1 1 1] Sphere tower
            (bind _returnvalue_2 (Game|SpawnActorfromClass "/Game/Blueprints/Actors/Towers/Parents/BP_SphereTower.BP_SphereTower_C" (Math|Transform|MakeTransform _towerpoint "0, 0, 0" "1,1,1") "Undefined" 0 0))
            (Default|Init _returnvalue_2 _towertype))
          (:NewEnumerator2
            (bind _returnvalue_3 (Game|SpawnActorfromClass "/Game/Blueprints/Actors/Towers/Parents/BP_SphereTower.BP_SphereTower_C" (Math|Transform|MakeTransform _towerpoint "0, 0, 0" "1,1,1") "Undefined" 0 0))
            (Default|Init _returnvalue_3 _towertype))
          (:NewEnumerator3
            (bind _returnvalue_4 (Game|SpawnActorfromClass "/Game/Blueprints/Actors/Towers/Parents/BP_ConeTower.BP_ConeTower_C" (Math|Transform|MakeTransform _towerpoint "0, 0, 0" "1,1,1") "Undefined" 0 0))
            (Default|Init _returnvalue_4 _towertype))
          (:NewEnumerator4
            (bind _returnvalue_5 (Game|SpawnActorfromClass "/Game/Blueprints/Actors/Towers/Parents/BP_SphereTower.BP_SphereTower_C" (Math|Transform|MakeTransform _towerpoint "0, 0, 0" "1,1,1") "Undefined" 0 0))
            (Default|Init _returnvalue_5 _towertype))
          (:NewEnumerator5
            ;[1 1 1] Base tower
            (bind _returnvalue_6 (Game|SpawnActorfromClass "/Game/Blueprints/Actors/Towers/Parents/BP_BaseTower.BP_BaseTower_C" (Math|Transform|MakeTransform _towerpoint "0, 0, 0" "1,1,1") "Undefined" 0 0))
            (Default|Init _returnvalue_6 _towertype))
          (:NewEnumerator6
            (bind _returnvalue_7 (Game|SpawnActorfromClass "/Game/Blueprints/Actors/Towers/Parents/BP_SphereTower.BP_SphereTower_C" (Math|Transform|MakeTransform _towerpoint "0, 0, 0" "1,1,1") "Undefined" 0 0))
            (Default|Init _returnvalue_7 _towertype))
          (:NewEnumerator7
            (bind _returnvalue_8 (Game|SpawnActorfromClass "/Game/Blueprints/Actors/Towers/Parents/BP_ConeTower.BP_ConeTower_C" (Math|Transform|MakeTransform _towerpoint "0, 0, 0" "1,1,1") "Undefined" 0 0))
            (Default|Init _returnvalue_8 _towertype))
          (:NewEnumerator8
            (bind _returnvalue_9 (Game|SpawnActorfromClass "/Game/Blueprints/Actors/Towers/Parents/BP_SphereTower.BP_SphereTower_C" (Math|Transform|MakeTransform _towerpoint "0, 0, 0" "1,1,1") "Undefined" 0 0))
            (Default|Init _returnvalue_9 _towertype))
          (:NewEnumerator9
            (bind _returnvalue_10 (Game|SpawnActorfromClass "/Game/Blueprints/Actors/Towers/Parents/BP_ConeTower.BP_ConeTower_C" (Math|Transform|MakeTransform _towerpoint "0, 0, 0" "1,1,1") "Undefined" 0 0))
            (Default|Init _returnvalue_10 _towertype)))
        (else
          (Variables|Default|SetInputCombination (Utilities|Struct|MakeSTRUCT_ElemToTowers "NewEnumerator2" "NewEnumerator0")))))))

(event Input|ActionEvents|InputActionElem_Earth
  (params (Key :type Key%20Structure))
  (bind _towerpoint (Variables|Default|GetTowerPoint))
  ;[1 1 1] Input combinations
  (:Pressed
    (if (Variables|Default|GetCanBuild)
      (if (Utilities|Enum|Equal(Enum) (.elem1 (Variables|Default|GetInputCombination)) "NewEnumerator0")
        (Variables|Default|SetInputCombination (Utilities|Struct|MakeSTRUCT_ElemToTowers (.elem1 (Variables|Default|GetInputCombination)) "NewEnumerator3"))
        (bind _towertype (CallFunction|InputtoTower (Variables|Default|GetInputCombination)))
        (switch Utilities|FlowControl|Switch|SwitchonENUM_Towers _towertype
          (:NewEnumerator0
            ;[1 1 1] Cone tower
            (bind _returnvalue (Game|SpawnActorfromClass "/Game/Blueprints/Actors/Towers/Parents/BP_ConeTower.BP_ConeTower_C" (Math|Transform|MakeTransform _towerpoint "0, 0, 0" "1,1,1") "Undefined" 0 0))
            (Default|Init _returnvalue _towertype))
          (:NewEnumerator1
            ;[1 1 1] Sphere tower
            (bind _returnvalue_2 (Game|SpawnActorfromClass "/Game/Blueprints/Actors/Towers/Parents/BP_SphereTower.BP_SphereTower_C" (Math|Transform|MakeTransform _towerpoint "0, 0, 0" "1,1,1") "Undefined" 0 0))
            (Default|Init _returnvalue_2 _towertype))
          (:NewEnumerator2
            (bind _returnvalue_3 (Game|SpawnActorfromClass "/Game/Blueprints/Actors/Towers/Parents/BP_SphereTower.BP_SphereTower_C" (Math|Transform|MakeTransform _towerpoint "0, 0, 0" "1,1,1") "Undefined" 0 0))
            (Default|Init _returnvalue_3 _towertype))
          (:NewEnumerator3
            (bind _returnvalue_4 (Game|SpawnActorfromClass "/Game/Blueprints/Actors/Towers/Parents/BP_ConeTower.BP_ConeTower_C" (Math|Transform|MakeTransform _towerpoint "0, 0, 0" "1,1,1") "Undefined" 0 0))
            (Default|Init _returnvalue_4 _towertype))
          (:NewEnumerator4
            (bind _returnvalue_5 (Game|SpawnActorfromClass "/Game/Blueprints/Actors/Towers/Parents/BP_SphereTower.BP_SphereTower_C" (Math|Transform|MakeTransform _towerpoint "0, 0, 0" "1,1,1") "Undefined" 0 0))
            (Default|Init _returnvalue_5 _towertype))
          (:NewEnumerator5
            ;[1 1 1] Base tower
            (bind _returnvalue_6 (Game|SpawnActorfromClass "/Game/Blueprints/Actors/Towers/Parents/BP_BaseTower.BP_BaseTower_C" (Math|Transform|MakeTransform _towerpoint "0, 0, 0" "1,1,1") "Undefined" 0 0))
            (Default|Init _returnvalue_6 _towertype))
          (:NewEnumerator6
            (bind _returnvalue_7 (Game|SpawnActorfromClass "/Game/Blueprints/Actors/Towers/Parents/BP_SphereTower.BP_SphereTower_C" (Math|Transform|MakeTransform _towerpoint "0, 0, 0" "1,1,1") "Undefined" 0 0))
            (Default|Init _returnvalue_7 _towertype))
          (:NewEnumerator7
            (bind _returnvalue_8 (Game|SpawnActorfromClass "/Game/Blueprints/Actors/Towers/Parents/BP_ConeTower.BP_ConeTower_C" (Math|Transform|MakeTransform _towerpoint "0, 0, 0" "1,1,1") "Undefined" 0 0))
            (Default|Init _returnvalue_8 _towertype))
          (:NewEnumerator8
            (bind _returnvalue_9 (Game|SpawnActorfromClass "/Game/Blueprints/Actors/Towers/Parents/BP_SphereTower.BP_SphereTower_C" (Math|Transform|MakeTransform _towerpoint "0, 0, 0" "1,1,1") "Undefined" 0 0))
            (Default|Init _returnvalue_9 _towertype))
          (:NewEnumerator9
            (bind _returnvalue_10 (Game|SpawnActorfromClass "/Game/Blueprints/Actors/Towers/Parents/BP_ConeTower.BP_ConeTower_C" (Math|Transform|MakeTransform _towerpoint "0, 0, 0" "1,1,1") "Undefined" 0 0))
            (Default|Init _returnvalue_10 _towertype)))
        (else
          (Variables|Default|SetInputCombination (Utilities|Struct|MakeSTRUCT_ElemToTowers "NewEnumerator3" "NewEnumerator0")))))))

(event Input|ActionEvents|InputActionElem_Fire
  (params (Key :type Key%20Structure))
  (bind _towerpoint (Variables|Default|GetTowerPoint))
  ;[1 1 1] Input combinations
  (:Pressed
    (if (Variables|Default|GetCanBuild)
      (if (Utilities|Enum|Equal(Enum) (.elem1 (Variables|Default|GetInputCombination)) "NewEnumerator0")
        (Variables|Default|SetInputCombination (Utilities|Struct|MakeSTRUCT_ElemToTowers (.elem1 (Variables|Default|GetInputCombination)) "NewEnumerator1"))
        (bind _towertype (CallFunction|InputtoTower (Variables|Default|GetInputCombination)))
        (switch Utilities|FlowControl|Switch|SwitchonENUM_Towers _towertype
          (:NewEnumerator0
            ;[1 1 1] Cone tower
            (bind _returnvalue (Game|SpawnActorfromClass "/Game/Blueprints/Actors/Towers/Parents/BP_ConeTower.BP_ConeTower_C" (Math|Transform|MakeTransform _towerpoint "0, 0, 0" "1,1,1") "Undefined" 0 0))
            (Default|Init _returnvalue _towertype))
          (:NewEnumerator1
            ;[1 1 1] Sphere tower
            (bind _returnvalue_2 (Game|SpawnActorfromClass "/Game/Blueprints/Actors/Towers/Parents/BP_SphereTower.BP_SphereTower_C" (Math|Transform|MakeTransform _towerpoint "0, 0, 0" "1,1,1") "Undefined" 0 0))
            (Default|Init _returnvalue_2 _towertype))
          (:NewEnumerator2
            (bind _returnvalue_3 (Game|SpawnActorfromClass "/Game/Blueprints/Actors/Towers/Parents/BP_SphereTower.BP_SphereTower_C" (Math|Transform|MakeTransform _towerpoint "0, 0, 0" "1,1,1") "Undefined" 0 0))
            (Default|Init _returnvalue_3 _towertype))
          (:NewEnumerator3
            (bind _returnvalue_4 (Game|SpawnActorfromClass "/Game/Blueprints/Actors/Towers/Parents/BP_ConeTower.BP_ConeTower_C" (Math|Transform|MakeTransform _towerpoint "0, 0, 0" "1,1,1") "Undefined" 0 0))
            (Default|Init _returnvalue_4 _towertype))
          (:NewEnumerator4
            (bind _returnvalue_5 (Game|SpawnActorfromClass "/Game/Blueprints/Actors/Towers/Parents/BP_SphereTower.BP_SphereTower_C" (Math|Transform|MakeTransform _towerpoint "0, 0, 0" "1,1,1") "Undefined" 0 0))
            (Default|Init _returnvalue_5 _towertype))
          (:NewEnumerator5
            ;[1 1 1] Base tower
            (bind _returnvalue_6 (Game|SpawnActorfromClass "/Game/Blueprints/Actors/Towers/Parents/BP_BaseTower.BP_BaseTower_C" (Math|Transform|MakeTransform _towerpoint "0, 0, 0" "1,1,1") "Undefined" 0 0))
            (Default|Init _returnvalue_6 _towertype))
          (:NewEnumerator6
            (bind _returnvalue_7 (Game|SpawnActorfromClass "/Game/Blueprints/Actors/Towers/Parents/BP_SphereTower.BP_SphereTower_C" (Math|Transform|MakeTransform _towerpoint "0, 0, 0" "1,1,1") "Undefined" 0 0))
            (Default|Init _returnvalue_7 _towertype))
          (:NewEnumerator7
            (bind _returnvalue_8 (Game|SpawnActorfromClass "/Game/Blueprints/Actors/Towers/Parents/BP_ConeTower.BP_ConeTower_C" (Math|Transform|MakeTransform _towerpoint "0, 0, 0" "1,1,1") "Undefined" 0 0))
            (Default|Init _returnvalue_8 _towertype))
          (:NewEnumerator8
            (bind _returnvalue_9 (Game|SpawnActorfromClass "/Game/Blueprints/Actors/Towers/Parents/BP_SphereTower.BP_SphereTower_C" (Math|Transform|MakeTransform _towerpoint "0, 0, 0" "1,1,1") "Undefined" 0 0))
            (Default|Init _returnvalue_9 _towertype))
          (:NewEnumerator9
            (bind _returnvalue_10 (Game|SpawnActorfromClass "/Game/Blueprints/Actors/Towers/Parents/BP_ConeTower.BP_ConeTower_C" (Math|Transform|MakeTransform _towerpoint "0, 0, 0" "1,1,1") "Undefined" 0 0))
            (Default|Init _returnvalue_10 _towertype)))
        (else
          (Variables|Default|SetInputCombination (Utilities|Struct|MakeSTRUCT_ElemToTowers "NewEnumerator1" "NewEnumerator0")))))))

(event Input|ActionEvents|InputActionElem_Water
  (params (Key :type Key%20Structure))
  (bind _towerpoint (Variables|Default|GetTowerPoint))
  ;[1 1 1] Input combinations
  (:Pressed
    (if (Variables|Default|GetCanBuild)
      (if (Utilities|Enum|Equal(Enum) (.elem1 (Variables|Default|GetInputCombination)) "NewEnumerator0")
        (Variables|Default|SetInputCombination (Utilities|Struct|MakeSTRUCT_ElemToTowers (.elem1 (Variables|Default|GetInputCombination)) "NewEnumerator4"))
        (bind _towertype (CallFunction|InputtoTower (Variables|Default|GetInputCombination)))
        (switch Utilities|FlowControl|Switch|SwitchonENUM_Towers _towertype
          (:NewEnumerator0
            ;[1 1 1] Cone tower
            (bind _returnvalue (Game|SpawnActorfromClass "/Game/Blueprints/Actors/Towers/Parents/BP_ConeTower.BP_ConeTower_C" (Math|Transform|MakeTransform _towerpoint "0, 0, 0" "1,1,1") "Undefined" 0 0))
            (Default|Init _returnvalue _towertype))
          (:NewEnumerator1
            ;[1 1 1] Sphere tower
            (bind _returnvalue_2 (Game|SpawnActorfromClass "/Game/Blueprints/Actors/Towers/Parents/BP_SphereTower.BP_SphereTower_C" (Math|Transform|MakeTransform _towerpoint "0, 0, 0" "1,1,1") "Undefined" 0 0))
            (Default|Init _returnvalue_2 _towertype))
          (:NewEnumerator2
            (bind _returnvalue_3 (Game|SpawnActorfromClass "/Game/Blueprints/Actors/Towers/Parents/BP_SphereTower.BP_SphereTower_C" (Math|Transform|MakeTransform _towerpoint "0, 0, 0" "1,1,1") "Undefined" 0 0))
            (Default|Init _returnvalue_3 _towertype))
          (:NewEnumerator3
            (bind _returnvalue_4 (Game|SpawnActorfromClass "/Game/Blueprints/Actors/Towers/Parents/BP_ConeTower.BP_ConeTower_C" (Math|Transform|MakeTransform _towerpoint "0, 0, 0" "1,1,1") "Undefined" 0 0))
            (Default|Init _returnvalue_4 _towertype))
          (:NewEnumerator4
            (bind _returnvalue_5 (Game|SpawnActorfromClass "/Game/Blueprints/Actors/Towers/Parents/BP_SphereTower.BP_SphereTower_C" (Math|Transform|MakeTransform _towerpoint "0, 0, 0" "1,1,1") "Undefined" 0 0))
            (Default|Init _returnvalue_5 _towertype))
          (:NewEnumerator5
            ;[1 1 1] Base tower
            (bind _returnvalue_6 (Game|SpawnActorfromClass "/Game/Blueprints/Actors/Towers/Parents/BP_BaseTower.BP_BaseTower_C" (Math|Transform|MakeTransform _towerpoint "0, 0, 0" "1,1,1") "Undefined" 0 0))
            (Default|Init _returnvalue_6 _towertype))
          (:NewEnumerator6
            (bind _returnvalue_7 (Game|SpawnActorfromClass "/Game/Blueprints/Actors/Towers/Parents/BP_SphereTower.BP_SphereTower_C" (Math|Transform|MakeTransform _towerpoint "0, 0, 0" "1,1,1") "Undefined" 0 0))
            (Default|Init _returnvalue_7 _towertype))
          (:NewEnumerator7
            (bind _returnvalue_8 (Game|SpawnActorfromClass "/Game/Blueprints/Actors/Towers/Parents/BP_ConeTower.BP_ConeTower_C" (Math|Transform|MakeTransform _towerpoint "0, 0, 0" "1,1,1") "Undefined" 0 0))
            (Default|Init _returnvalue_8 _towertype))
          (:NewEnumerator8
            (bind _returnvalue_9 (Game|SpawnActorfromClass "/Game/Blueprints/Actors/Towers/Parents/BP_SphereTower.BP_SphereTower_C" (Math|Transform|MakeTransform _towerpoint "0, 0, 0" "1,1,1") "Undefined" 0 0))
            (Default|Init _returnvalue_9 _towertype))
          (:NewEnumerator9
            (bind _returnvalue_10 (Game|SpawnActorfromClass "/Game/Blueprints/Actors/Towers/Parents/BP_ConeTower.BP_ConeTower_C" (Math|Transform|MakeTransform _towerpoint "0, 0, 0" "1,1,1") "Undefined" 0 0))
            (Default|Init _returnvalue_10 _towertype)))
        (else
          (Variables|Default|SetInputCombination (Utilities|Struct|MakeSTRUCT_ElemToTowers "NewEnumerator4" "NewEnumerator0")))))))

(event Input|AxisEvents|InputAxisMoveForward
  (params (AxisValue :type Float%20%28single-precision%29))
  ;[1 0.1788 0] Moving controls
  (Pawn|Input|AddMovementInput (Math|Vector|GetForwardVector (Variables|Character|GetMesh)) AxisValue false))

(event Input|AxisEvents|InputAxisMoveRight
  (params (AxisValue :type Float%20%28single-precision%29))
  ;[1 0.1788 0] Moving controls
  (Pawn|Input|AddMovementInput (Math|Vector|GetRightVector (Variables|Character|GetMesh)) AxisValue false))

(fn ConstructionScript
  (Utilities|Map|Add (Variables|Default|GetDicTowers) (Utilities|Struct|MakeSTRUCT_ElemToTowers "NewEnumerator1" "NewEnumerator1") "")
  (Utilities|Map|Add (Variables|Default|GetDicTowers) (Utilities|Struct|MakeSTRUCT_ElemToTowers "NewEnumerator1" "NewEnumerator2") "NewEnumerator1")
  (Utilities|Map|Add (Variables|Default|GetDicTowers) (Utilities|Struct|MakeSTRUCT_ElemToTowers "NewEnumerator2" "NewEnumerator2") "NewEnumerator2")
  (Utilities|Map|Add (Variables|Default|GetDicTowers) (Utilities|Struct|MakeSTRUCT_ElemToTowers "NewEnumerator2" "NewEnumerator4") "NewEnumerator3")
  (Utilities|Map|Add (Variables|Default|GetDicTowers) (Utilities|Struct|MakeSTRUCT_ElemToTowers "NewEnumerator4" "NewEnumerator3") "NewEnumerator5")
  (Utilities|Map|Add (Variables|Default|GetDicTowers) (Utilities|Struct|MakeSTRUCT_ElemToTowers "NewEnumerator3" "NewEnumerator3") "NewEnumerator6")
  (Utilities|Map|Add (Variables|Default|GetDicTowers) (Utilities|Struct|MakeSTRUCT_ElemToTowers "NewEnumerator3" "NewEnumerator1") "NewEnumerator7")
  (Utilities|Map|Add (Variables|Default|GetDicTowers) (Utilities|Struct|MakeSTRUCT_ElemToTowers "NewEnumerator2" "NewEnumerator3") "NewEnumerator8")
  (Utilities|Map|Add (Variables|Default|GetDicTowers) (Utilities|Struct|MakeSTRUCT_ElemToTowers "NewEnumerator4" "NewEnumerator1") "NewEnumerator9"))

(fn InputtoTower
  (params (InputCombination :type STRUCT%20Elem%20to%20Towers%20Structure))
  (switch Utilities|FlowControl|Switch|SwitchonENUM_Elem (.elem1 InputCombination)
    (:NewEnumerator1
      (switch Utilities|FlowControl|Switch|SwitchonENUM_Elem (.elem2 InputCombination)
        (:NewEnumerator1
          (return "NewEnumerator0"))
        (:NewEnumerator2
          _)
        (:NewEnumerator3
          (return "NewEnumerator7"))
        (:NewEnumerator4
          (return "NewEnumerator9"))))
    (:NewEnumerator2
      (switch Utilities|FlowControl|Switch|SwitchonENUM_Elem (.elem2 InputCombination)
        (:NewEnumerator1
          _)
        (:NewEnumerator2
          (return "NewEnumerator2"))
        (:NewEnumerator3
          (return "NewEnumerator8"))
        (:NewEnumerator4
          (return "NewEnumerator3"))))
    (:NewEnumerator3
      (switch Utilities|FlowControl|Switch|SwitchonENUM_Elem (.elem2 InputCombination)
        (:NewEnumerator1
          (return "NewEnumerator7"))
        (:NewEnumerator2
          (return "NewEnumerator2"))
        (:NewEnumerator3
          (return "NewEnumerator6"))
        (:NewEnumerator4
          (return "NewEnumerator5"))))
    (:NewEnumerator4
      (switch Utilities|FlowControl|Switch|SwitchonENUM_Elem (.elem2 InputCombination)
        (:NewEnumerator1
          (return "NewEnumerator9"))
        (:NewEnumerator2
          (return "NewEnumerator3"))
        (:NewEnumerator3
          (return "NewEnumerator5"))
        (:NewEnumerator4
          (return "NewEnumerator4")))))
  (return "NewEnumerator1"))