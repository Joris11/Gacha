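; Player-controlled hub character with a paper flipbook sprite that moves along its mesh axes and flips with horizontal input.
; Confirm near an interactable starts the main-menu HUD's credits, Elem_Fire stops them, and Elem_Earth at an exit loads the next level.
; InputToTower maps two-element combinations to tower types, uncalled here and order-independent except Air/Earth, where Earth-Air returns the Air-Air result.
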(event Custom|AnimWalk
  ;[1 1 1] Input converted to tower type
  ;;[1 1 1] Ends previous animation
  (Variables|Components|SetSpeed 1.0)
  (Utilities|FlowControl|Delay (+ (Class|PaperFlipbookComponent|GetFlipbookLength (Variables|Default|GetPaperFlipbook)) 0.15))
  (Sprite|SetFlipbook (Variables|Default|GetPaperFlipbook) "/Game/Anim/ANIM_Walk.ANIM_Walk"))

(event Custom|AnimIdle
  ;[1 1 1] Input converted to tower type
)

(event EventBeginPlay
  ;[1 1 1] Input converted to tower type
  (Variables|Default|SetHUDREF (.AsHUD%20Main%20Menu (Utilities|Casting|CastToHUD_MainMenu (HUD|GetHUD (Game|GetPlayerController 0))))))

(event Input|ActionEvents|InputActionConfirm
  (params (Key :type Key%20Structure))
  ;[1 1 1] Input converted to tower type
  (:Pressed
    (if (Variables|Components|GetOverlappingInteract)
      (Default|StartCreditScore (Variables|Default|GetHUDREF))
      (Audio|PlaySoundatLocation (Variables|Default|GetOpenBook) "0, 0, 0"))))

(event Input|ActionEvents|InputActionElem_Fire
  (params (Key :type Key%20Structure))
  ;[1 1 1] Input converted to tower type
  (:Pressed
    (Default|CallSTOPCredits (Variables|Default|GetHUDREF))))

(event Input|ActionEvents|InputActionElem_Earth
  (params (Key :type Key%20Structure))
  ;[1 1 1] Input converted to tower type
  (:Pressed
    (if (Variables|Default|GetOverlappingExit)
      (Game|OpenLevel(byName) (Utilities|String|StringToName (Utilities|String|Append "Levelneutre" (Variables|Default|GetNextLevelDenom))))
      (Audio|PlaySoundatLocation (Variables|Default|GetOpenDoor) "0, 0, 0"))))

(event Input|AxisEvents|InputAxisMoveForward
  (params (AxisValue :type Float%20%28single-precision%29))
  ;[1 1 1] Input converted to tower type
  ;;[1 0.1788 0] Moving controls
  (Pawn|Input|AddMovementInput (Math|Vector|GetForwardVector (Variables|Character|GetMesh)) (* (Variables|Components|GetSpeed) AxisValue) false)
  (if (not (> AxisValue 0.2))
    (if (< AxisValue -0.2)
      _)))

(event Input|AxisEvents|InputAxisMoveRight
  (params (AxisValue :type Float%20%28single-precision%29))
  ;[1 1 1] Input converted to tower type
  ;;[1 0.1788 0] Moving controls
  (Pawn|Input|AddMovementInput (Math|Vector|GetRightVector (Variables|Character|GetMesh)) (* (Variables|Components|GetSpeed) AxisValue) false)
  (if (> AxisValue 0.2)
    (Transformation|SetRelativeRotation (Variables|Default|GetPaperFlipbook) "0.000000,-90.000000,90.000000" false false)
    (elif (< AxisValue -0.2)
      (Transformation|SetRelativeRotation (Variables|Default|GetPaperFlipbook) "180.000000,-90.000000,90.000000" false false))))

(fn ConstructionScript)

(fn InputtoTower
  (params (InputCombination :type STRUCT%20Elem%20to%20Towers%20Structure))
  (switch Utilities|FlowControl|Switch|SwitchonENUM_Elem (.elem1 InputCombination)
    (:NewEnumerator1
      (switch Utilities|FlowControl|Switch|SwitchonENUM_Elem (.elem2 InputCombination)
        (:NewEnumerator1
          (return "NewEnumerator0"))
        (:NewEnumerator2
          _)
        (:NewEnumerator3
          (return "NewEnumerator7"))
        (:NewEnumerator4
          (return "NewEnumerator9"))))
    (:NewEnumerator2
      (switch Utilities|FlowControl|Switch|SwitchonENUM_Elem (.elem2 InputCombination)
        (:NewEnumerator1
          _)
        (:NewEnumerator2
          (return "NewEnumerator2"))
        (:NewEnumerator3
          (return "NewEnumerator8"))
        (:NewEnumerator4
          (return "NewEnumerator3"))))
    (:NewEnumerator3
      (switch Utilities|FlowControl|Switch|SwitchonENUM_Elem (.elem2 InputCombination)
        (:NewEnumerator1
          (return "NewEnumerator7"))
        (:NewEnumerator2
          (return "NewEnumerator2"))
        (:NewEnumerator3
          (return "NewEnumerator6"))
        (:NewEnumerator4
          (return "NewEnumerator5"))))
    (:NewEnumerator4
      (switch Utilities|FlowControl|Switch|SwitchonENUM_Elem (.elem2 InputCombination)
        (:NewEnumerator1
          (return "NewEnumerator9"))
        (:NewEnumerator2
          (return "NewEnumerator3"))
        (:NewEnumerator3
          (return "NewEnumerator5"))
        (:NewEnumerator4
          (return "NewEnumerator4")))))
  (return "NewEnumerator1"))