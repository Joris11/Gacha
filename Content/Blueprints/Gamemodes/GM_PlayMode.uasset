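; Game mode for play levels that spawns a base tower and schedules rat hordes.
; On BeginPlay it reads level influence from the game instance, gathers rat spawn points and waits before the first horde.
; ChangeSpawnRat triggers a horde on one of three random spawn points, then re-calls itself after a delay with an incremented index, stopping at five.
; Direct rat spawning is unconnected, and SpawnRatWave is empty.
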(event Custom|Change%20Spawn%20Rat
  (bind _asbp_rat_spawn_point (Utilities|Casting|CastToBP_RatSpawnPoint (Utilities|Array|Get(acopy) (Variables|Default|GetspawnRatIndex) (Math|Random|RandomIntegerinRange 0 2))))
  (Default|Horde1 _asbp_rat_spawn_point (Variables|Default|GetnextHorde))
  (if (not (== (+ (Variables|Default|GetcompteurHorde) 1) 5))
    (Utilities|FlowControl|Delay 1e+01)
    (bind _output_get (Variables|Default|SetnextHorde (+ (Variables|Default|GetnextHorde) 1)))
    (if (not (== _output_get 5))
      (CallFunction|ChangeSpawnRat))))

(event Custom|InitializeProperties
  ;[1 1 1] Init
  (bind _asbp_game_instance (Utilities|Casting|CastToBP_GameInstance (Game|GetGameInstance)))
  (Variables|Components|SetM%20LevelInfluence (Variables|/Game/Blueprints/GameInstances/BP_GameInstance.BP_GameInstance_C|GetM%20LevelInfluence _asbp_game_instance)))

(event EventBeginPlay
  (CallFunction|InitializeProperties)
  (bind _returnvalue (Game|SpawnActorfromClass "/Game/Blueprints/Actors/Towers/Parents/BP_BaseTower.BP_BaseTower_C" (Math|Transform|MakeTransform "0, 0, 0" "0, 0, 0" "1,1,1") "Undefined" 0 0))
  (Default|Init _returnvalue "NewEnumerator2")
  (bind _outactors (Actor|GetAllActorsOfClass "/Game/Blueprints/Actors/GameplayElement/BP_RatSpawnPoint.BP_RatSpawnPoint_C"))
  (Variables|Default|SetspawnRatIndex _outactors)
  (Utilities|FlowControl|Delay 15.0)
  (Utilities|FlowControl|Delay 0.2)
  (CallFunction|ChangeSpawnRat))

(event EventTick
  (params (DeltaSeconds :type Float%20%28single-precision%29)))

(fn ConstructionScript)

(fn SpawnRatWave)

(fn GetRandomRat
  (bind _m_ratstemplate (Variables|Components|GetM%20RatsTemplate))
  (return (.type (Utilities|Array|Get(acopy) (.rats _m_ratstemplate) (Math|Random|RandomIntegerinRange 0 (- (Utilities|Array|Length (.rats _m_ratstemplate)) 1))))))