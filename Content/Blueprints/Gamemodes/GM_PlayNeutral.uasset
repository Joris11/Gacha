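; GM_PlayNeutral is a game mode that stages the opening ambient soundscape for neutral play.
; After the parent BeginPlay, it starts a peaceful ambience, then, after a delay, fades in general and two thunder layers on separate audio tracks.
; A fast bell plays on the event track shortly afterward, then the peaceful layer slowly fades out.
; Tick accumulates CurrentTime but otherwise only holds an empty branch.
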(event EventBeginPlay
  (bind _track_ambient02 (Variables|Default|GetTrack_Ambient02))
  (bind _track_ambient03 (Variables|Default|GetTrack_Ambient03))
  (bind _track_event (Variables|Default|GetTrack_Event))
  (bind _track_ambient01 (Variables|Default|GetTrack_Ambient01))
  (bind _track_other (Variables|Default|GetTrack_Other))
  (|CallParentFunction)
  (Audio|Components|Audio|SetSound _track_other "/Game/Sounds/Ambiances/Classic/Ambiance-Neutre-Paisible.Ambiance-Neutre-Paisible")
  (Audio|Components|Audio|Play _track_other 0.0)
  (Utilities|FlowControl|Delay 1e+01)
  (Audio|Components|Audio|SetSound _track_ambient01 "/Game/Sounds/Ambiances/Classic/Ambiance-Neutre-General_Cue.Ambiance-Neutre-General_Cue")
  (Audio|Components|Audio|Play _track_ambient01 0.0)
  (Audio|Components|Audio|FadeIn _track_ambient01 1e+01 1.0 0.0 :!class /Script/Engine.AudioComponent)
  (Audio|Components|Audio|SetSound _track_ambient02 "/Game/Sounds/Ambiances/Classic/Ambiance-Neutre-Thunder-1_Cue.Ambiance-Neutre-Thunder-1_Cue")
  (Audio|Components|Audio|Play _track_ambient02 0.0)
  (Audio|Components|Audio|FadeIn _track_ambient02 1e+01 1.0 0.0 :!class /Script/Engine.AudioComponent)
  (Audio|Components|Audio|SetSound _track_ambient03 "/Game/Sounds/Ambiances/Classic/Ambiance-Neutre-Thunder-2_Cue.Ambiance-Neutre-Thunder-2_Cue")
  (Audio|Components|Audio|Play _track_ambient03 0.0)
  (Audio|Components|Audio|FadeIn _track_ambient03 1e+01 1.0 0.0 :!class /Script/Engine.AudioComponent)
  (Utilities|FlowControl|Delay 5.0)
  (Audio|Components|Audio|SetSound _track_event "/Game/Sounds/Ambiances/Classic/Ambiance-Bell-Fast.Ambiance-Bell-Fast")
  (Audio|Components|Audio|Play _track_event 0.0)
  (Utilities|FlowControl|Delay 5.0)
  (Audio|Components|Audio|FadeOut (Variables|Default|GetTrack_Other) 2e+01 0.0 :!class /Script/Engine.AudioComponent))

(event EventTick
  (params (DeltaSeconds :type Float%20%28single-precision%29))
  (Variables|Default|SetcurrentTime (+ (Variables|Default|GetcurrentTime) DeltaSeconds))
  (if true
    _))

(fn ConstructionScript
  (|CallParentFunction))