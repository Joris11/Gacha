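; GM_PlayWind is a game mode Blueprint that sets up wind ambience when play begins.
; After the parent BeginPlay, it assigns two general wind cues to the two ambient tracks and starts them together.
; Following a fixed delay, it plays a one-shot trigger of a fast bell sound on the separate event track.
; The construction script only calls its parent.
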(event EventBeginPlay
  (bind _track_ambient02 (Variables|Default|GetTrack_Ambient02))
  (bind _track_event (Variables|Default|GetTrack_Event))
  (bind _track_ambient01 (Variables|Default|GetTrack_Ambient01))
  (|CallParentFunction)
  (Audio|Components|Audio|SetSound _track_ambient01 "/Game/Sounds/Ambiances/Classic/Ambiance-Wind-General-1_Cue.Ambiance-Wind-General-1_Cue")
  (Audio|Components|Audio|Play _track_ambient01 0.0)
  (Audio|Components|Audio|SetSound _track_ambient02 "/Game/Sounds/Ambiances/Classic/Ambiance-Wind-General-2_Cue.Ambiance-Wind-General-2_Cue")
  (Audio|Components|Audio|Play _track_ambient02 0.0)
  (Utilities|FlowControl|Delay 15.0)
  (Audio|Components|Audio|SetSound _track_event "/Game/Sounds/Ambiances/Classic/Ambiance-Bell-Fast.Ambiance-Bell-Fast")
  (Audio|Components|Audio|Play _track_event 0.0))

(fn ConstructionScript
  (|CallParentFunction))