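; Base enemy rat pawn that walks a route through the level's TargetPoint actors.
; Init picks the rat's data from RatsTemplate by type, with upgraded entries for Flying, Tank, Speed and Ninja.
; BeginPlay gathers all TargetPoints in unsorted GetAllActorsOfClass order, and AIPAth chains AIMoveTo calls, advancing the waypoint index on each success.
; Logic to notify BP_Goal and stop movement is disconnected from the empty overlap event.
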(event Custom|AIPAth
  (bind _targetpoint (Variables|Default|GetTargetPoint))
  (AI|AIMoveTo self "0, 0, 0" (Utilities|Array|Get(acopy) _targetpoint (Variables|Default|GetIndexWayPoint)) 1.0 false
    (:OnSuccess
      (bind _output_get (Variables|Default|SetIndexWayPoint (+ (Variables|Default|GetIndexWayPoint) 1)))
      (if (not (> _output_get (Utilities|Array|Length _targetpoint)))
        (CallFunction|AIPAth)))))

(event Custom|Init
  (params (RatType :type ENUM_RatType%20Enum :default "NewEnumerator0") (IsUpgraded :type Boolean))
  (bind _ratstemplate (Variables|Templates|GetratsTemplate))
  ;[1 1 1] Rat init conversion
  (switch Utilities|FlowControl|Switch|SwitchonENUM_RatType RatType
    (:NewEnumerator0
      (Variables|Default|SetratType (Utilities|Array|Get(acopy) (.rats _ratstemplate))))
    (:NewEnumerator5
      (Variables|Default|SetratType (Utilities|Array|Get(acopy) (.rats _ratstemplate) 6)))
    (:NewEnumerator1
      (if IsUpgraded
        (Variables|Default|SetratType (Utilities|Array|Get(acopy) (.rats _ratstemplate) 7))
        (else
          (Variables|Default|SetratType (Utilities|Array|Get(acopy) (.rats _ratstemplate) 1)))))
    (:NewEnumerator6
      (if IsUpgraded
        (Variables|Default|SetratType (Utilities|Array|Get(acopy) (.rats _ratstemplate) 8))
        (else
          (Variables|Default|SetratType (Utilities|Array|Get(acopy) (.rats _ratstemplate) 2)))))
    (:NewEnumerator2
      (if IsUpgraded
        (Variables|Default|SetratType (Utilities|Array|Get(acopy) (.rats _ratstemplate) 9))
        (else
          (Variables|Default|SetratType (Utilities|Array|Get(acopy) (.rats _ratstemplate) 3)))))
    (:NewEnumerator3
      (if IsUpgraded
        (Variables|Default|SetratType (Utilities|Array|Get(acopy) (.rats _ratstemplate) 10))
        (else
          (Variables|Default|SetratType (Utilities|Array|Get(acopy) (.rats _ratstemplate) 4)))))
    (:NewEnumerator4
      (Variables|Default|SetratType (Utilities|Array|Get(acopy) (.rats _ratstemplate) 5)))))

(event Collision|EventActorBeginOverlap
  (params (OtherActor :type Actor%20Object%20Reference))
  ;[1 0 0.8488] STOP AT GOAL
)

(event EventTick
  (params (DeltaSeconds :type Float%20%28single-precision%29)))

(event EventBeginPlay
  ;[0 1 0.995] IA MOVE
  (bind _outactors (Actor|GetAllActorsOfClass "/Script/Engine.TargetPoint"))
  (for _array_element _outactors
    (Utilities|Array|Add (Variables|Default|GetTargetPoint) _array_element))
  (CallFunction|AIPAth))

(fn ConstructionScript)