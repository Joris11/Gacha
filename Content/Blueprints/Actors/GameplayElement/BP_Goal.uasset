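; BP_Goal is the goal actor that rats attack and that the player enters to return to the HUB level once a wave ends.
; Overlapping rats subtract their RatType damage from HP in BP_GameInstance and are destroyed.
; A player overlap after DPS reports WaveEnd adds HP times Wave to Score, then triggers OpenLevel by timer.
; Both paths update text on a HUB widget created at BeginPlay.
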(event Custom|OpenLevel
  ;[1 1 1] Go into hub
  (Game|OpenLevel(byName) "HUB"))

(event Collision|EventActorBeginOverlap
  (params (OtherActor :type Actor%20Object%20Reference))
  (bind _returnvalue (Utilities|GetClass OtherActor))
  (bind _mongameinstance (Variables|Default|GetmonGameInstance))
  (bind _mongameinstance_2 (Variables|Default|GetmonGameInstance))
  ;[1 1 1] Go into hub
  (if (== _returnvalue "/Game/Blueprints/Players/BP_Player.BP_Player_C")
    (Utilities|Casting|CastToBP_Player OtherActor)
    (if (Variables|/Game/Blueprints/Actors/Towers/DPSMeter.DPSMeter_C|GetWaveEnd (Variables|Default|GetDPS))
      ;[1 1 1] Set score increment at the end of wave
      (bind _output_get (Variables|/Game/Blueprints/GameInstances/BP_GameInstance.BP_GameInstance_C|SetScore _mongameinstance (+ (Variables|/Game/Blueprints/GameInstances/BP_GameInstance.BP_GameInstance_C|GetScore _mongameinstance) (* (Variables|/Game/Blueprints/GameInstances/BP_GameInstance.BP_GameInstance_C|GetHP _mongameinstance) (Variables|/Game/Blueprints/GameInstances/BP_GameInstance.BP_GameInstance_C|GetWave _mongameinstance)))))
      (Rendering|Components|TextRender|SetText (Variables|/Game/Blueprints/Widgets/HUB.HUB_C|GetScore (Variables|Default|GetHUBWidget)) (Utilities|Text|ToText(String) (Utilities|String|Append (Variables|Default|GetScoreText) (Utilities|String|ToString(Integer) _output_get))))
      (Utilities|Time|SetTimerbyFunctionName 0 "OpenLevel" 0.0))
    (else
      ;[1 1 1] Receive rat damage
      (if (== _returnvalue "/Game/Blueprints/Actors/Enemy/BP_BaseRats.BP_BaseRats_C")
        (bind _asbp_base_rats (Utilities|Casting|CastToBP_BaseRats OtherActor))
        (bind _output_get_2 (Variables|/Game/Blueprints/GameInstances/BP_GameInstance.BP_GameInstance_C|SetHP _mongameinstance_2 (- (Variables|/Game/Blueprints/GameInstances/BP_GameInstance.BP_GameInstance_C|GetHP _mongameinstance_2) (Math|Float|Truncate (.damage (Variables|/Game/Blueprints/Actors/Enemy/BP_BaseRats.BP_BaseRats_C|GetratType _asbp_base_rats))))))
        (Actor|DestroyActor OtherActor)
        (Rendering|Components|TextRender|SetText (Variables|/Game/Blueprints/Widgets/HUB.HUB_C|GetLives (Variables|Default|GetHUBWidget)) (Utilities|Text|ToText(String) (Utilities|String|Append (Variables|Default|GetLivesText) (Utilities|String|ToString(Integer) _output_get_2))))))))

(event EventBeginPlay
  ;[1 1 1] Game Instance + widget
  (Utilities|FlowControl|Sequence
    (:then_0
      (bind _returnvalue (UserInterface|CreateWidget "/Game/Blueprints/Widgets/HUB.HUB_C"))
      (Variables|Default|SetHUBWidget _returnvalue))
    (:then_1
      (bind _asbp_game_instance (Utilities|Casting|CastToBP_GameInstance (Game|GetGameInstance)))
      (Variables|Default|SetmonGameInstance _asbp_game_instance))))

(fn ConstructionScript)