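; BP_RatSpawnPoint is a placeable actor that spawns a single BP_BaseRats at its own transform on BeginPlay.
; SpawnRatType picks a random rat type from the MRatsTemplate Rats list in GM_PlayMode, with an inclusive upper bound equal to the array length, one past the last index.
; The Init call that would pass that type to the spawned rat is disconnected, so the chosen type is never applied.
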(event EventBeginPlay
  (bind _rattype (CallFunction|SpawnRatType))
  (bind _returnvalue (Game|SpawnActorfromClass "/Game/Blueprints/Actors/Enemy/BP_BaseRats.BP_BaseRats_C" (Transformation|GetWorldTransform (Variables|Default|GetDefaultSceneRoot)) "AlwaysSpawn" 0 0)))

(event Collision|EventActorBeginOverlap
  (params (OtherActor :type Actor%20Object%20Reference)))

(event EventTick
  (params (DeltaSeconds :type Float%20%28single-precision%29)))

(fn ConstructionScript)

(fn SpawnRatType
  (bind _asgm_play_mode (Utilities|Casting|CastToGM_PlayMode (Game|GetGameMode)))
  (return (.type (Utilities|Array|Get(acopy) (.rats (Variables|/Game/Blueprints/Gamemodes/GM_PlayMode.GM_PlayMode_C|GetM%20RatsTemplate _asgm_play_mode)) (Math|Random|RandomIntegerinRange 0 (Utilities|Array|Length (.rats (Variables|/Game/Blueprints/Gamemodes/GM_PlayMode.GM_PlayMode_C|GetM%20RatsTemplate _asgm_play_mode))))))))