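; BP_InteractionTrigger is a trigger actor that shows a crystal prompt and hands the player a tower spot to interact with.
; On overlap it toggles the alpha of three sprites and sets BP_Player's overlap references and tower point from MTowerSpot.
; FirstInput and SecondInput events restyle the lower and upper triangles by chosen element (Fire, Air, Earth, Water), swapping sprite and relative position.
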(event OnComponentBeginOverlap(Trigger)
  (params (OverlappedComponent :type Primitive%20Component%20Object%20Reference) (OtherActor :type Actor%20Object%20Reference) (OtherComp :type Primitive%20Component%20Object%20Reference) (OtherBodyIndex :type Integer) (bFromSweep :type Boolean) (SweepResult :type Hit%20Result%20Structure%20%28by%20ref%29))
  ;[1 1 1] Show
  (bind _asbp_player (Utilities|Casting|CastToBP_Player OtherActor))
  (CallFunction|Display true)
  (Variables|/Game/Blueprints/Players/BP_Player.BP_Player_C|SetOverlappedInteract _asbp_player self)
  (Variables|/Game/Blueprints/Players/BP_Player.BP_Player_C|SetOverlappingInteract _asbp_player true)
  (Variables|/Game/Blueprints/Players/BP_Player.BP_Player_C|SetTowerPoint _asbp_player (Transformation|GetActorLocation (Variables|Components|GetM%20TowerSpot))))

(event OnComponentEndOverlap(Trigger)
  (params (OverlappedComponent :type Primitive%20Component%20Object%20Reference) (OtherActor :type Actor%20Object%20Reference) (OtherComp :type Primitive%20Component%20Object%20Reference) (OtherBodyIndex :type Integer))
  ;[1 1 1] Hide
  (bind _asbp_player (Utilities|Casting|CastToBP_Player OtherActor))
  (CallFunction|Display false)
  (Variables|/Game/Blueprints/Players/BP_Player.BP_Player_C|SetOverlappingInteract _asbp_player false))

(event Custom|SecondInput
  (params (2ndInput :type ENUM_Elem%20Enum :default "NewEnumerator0"))
  (bind _triangle1 (Variables|Default|GetTriangle1))
  (bind _m_trianglepositions (Variables|Components|GetM%20TrianglePositions))
  ;[1 1 1] Applies transform
  (switch Utilities|FlowControl|Switch|SwitchonENUM_Elem 2ndInput
    (:NewEnumerator1
      (Rendering|Components|Sprite|SetSprite _triangle1 "/Game/Textures/InputInteraction/Cristal_rouge_haut_Sprite.Cristal_Rouge_Haut_Sprite")
      (Transformation|SetRelativeLocation _triangle1 (Utilities|Array|Get(acopy) _m_trianglepositions 4) false false))
    (:NewEnumerator2
      (Rendering|Components|Sprite|SetSprite _triangle1 "/Game/Textures/InputInteraction/Cristal_jaune_haut_Sprite.Cristal_Jaune_Haut_Sprite")
      (Transformation|SetRelativeLocation _triangle1 (Utilities|Array|Get(acopy) _m_trianglepositions 5) false false))
    (:NewEnumerator3
      (Rendering|Components|Sprite|SetSprite _triangle1 "/Game/Textures/InputInteraction/Cristal_vert_haut_Sprite.Cristal_Vert_Haut_Sprite")
      (Transformation|SetRelativeLocation _triangle1 (Utilities|Array|Get(acopy) _m_trianglepositions 6) false false))
    (:NewEnumerator4
      (Rendering|Components|Sprite|SetSprite _triangle1 "/Game/Textures/InputInteraction/Cristal_bleu_haut_Sprite.Cristal_Bleu_Haut_Sprite")
      (Transformation|SetRelativeLocation _triangle1 (Utilities|Array|Get(acopy) _m_trianglepositions 7) false false))))

(event Custom|FirstInput
  (params (1stInput :type ENUM_Elem%20Enum :default "NewEnumerator0"))
  (bind _m_trianglepositions (Variables|Components|GetM%20TrianglePositions))
  (bind _triangle2 (Variables|Default|GetTriangle2))
  ;[1 1 1] Applies transform
  (switch Utilities|FlowControl|Switch|SwitchonENUM_Elem 1stInput
    (:NewEnumerator1
      (Rendering|Components|Sprite|SetSprite _triangle2 "/Game/Textures/InputInteraction/Cristal_rouge_bas_Sprite.Cristal_Rouge_Bas_Sprite")
      (Transformation|SetRelativeLocation _triangle2 (Utilities|Array|Get(acopy) _m_trianglepositions) false false))
    (:NewEnumerator2
      (Rendering|Components|Sprite|SetSprite _triangle2 "/Game/Textures/InputInteraction/Cristal_jaune_bas_Sprite.Cristal_Jaune_Bas_Sprite")
      (Transformation|SetRelativeLocation _triangle2 (Utilities|Array|Get(acopy) _m_trianglepositions 1) false false))
    (:NewEnumerator3
      (Rendering|Components|Sprite|SetSprite _triangle2 "/Game/Textures/InputInteraction/Cristal_vert_bas_Sprite.Cristal_Vert_Bas_Sprite")
      (Transformation|SetRelativeLocation _triangle2 (Utilities|Array|Get(acopy) _m_trianglepositions 2) false false))
    (:NewEnumerator4
      (Rendering|Components|Sprite|SetSprite _triangle2 "/Game/Textures/InputInteraction/Cristal_bleu_bas_Sprite.Cristal_Bleu_Bas_Sprite")
      (Transformation|SetRelativeLocation _triangle2 (Utilities|Array|Get(acopy) _m_trianglepositions 3) false false))))

(event Custom|Display
  (params (Show :type Boolean))
  (bind _losange (Variables|Default|GetLosange))
  (bind _losange_2 (Variables|Default|GetLosange))
  (bind _spritecolor (Variables|/Script/Paper2D.PaperSpriteComponent|GetSpriteColor _losange))
  (bind _spritecolor_2 (Variables|/Script/Paper2D.PaperSpriteComponent|GetSpriteColor _losange_2))
  ;[1 1 1] DISPLAY
  (if Show
    (Sprite|SetSpriteColor _losange (Utilities|Struct|MakeLinearColor (.r _spritecolor) (.g _spritecolor) (.b _spritecolor) 1.0))
    (Sprite|SetSpriteColor (Variables|Default|GetTriangle1) (Utilities|Struct|MakeLinearColor (.r _spritecolor) (.g _spritecolor) (.b _spritecolor) 1.0))
    (Sprite|SetSpriteColor (Variables|Default|GetTriangle2) (Utilities|Struct|MakeLinearColor (.r _spritecolor) (.g _spritecolor) (.b _spritecolor) 1.0))
    (else
      (Sprite|SetSpriteColor _losange_2 (Utilities|Struct|MakeLinearColor (.r _spritecolor_2) (.g _spritecolor_2) (.b _spritecolor_2) 0.0))
      (Sprite|SetSpriteColor (Variables|Default|GetTriangle1) (Utilities|Struct|MakeLinearColor (.r _spritecolor_2) (.g _spritecolor_2) (.b _spritecolor_2) 0.0))
      (Sprite|SetSpriteColor (Variables|Default|GetTriangle2) (Utilities|Struct|MakeLinearColor (.r _spritecolor_2) (.g _spritecolor_2) (.b _spritecolor_2) 0.0)))))

(fn ConstructionScript)