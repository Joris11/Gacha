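; BP_Hightlightable is a main menu actor that highlights and triggers a menu action when the player overlaps it.
; On begin overlap it switches its sprite to the highlighted one and, based on MFunctionToCall, tells HUD_MainMenu to show the upgrade menu or start the credits.
; End overlap only restores the neutral sprite, which the construction script also applies when valid.
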(event Collision|EventActorBeginOverlap
  (params (OtherActor :type Actor%20Object%20Reference))
  (Utilities|Casting|CastToBP_Player OtherActor)
  (Rendering|Components|Sprite|SetSprite (Variables|Default|GetSprite) (Variables|Components|GetM%20HighlightedSprite))
  (bind _ashud_main_menu (Utilities|Casting|CastToHUD_MainMenu (HUD|GetHUD (Game|GetPlayerController 0))))
  (switch Utilities|FlowControl|Switch|SwitchonENUM_HudFunctions (Variables|Components|GetM%20FunctionToCall)
    (:NewEnumerator0
      (Default|DisplayUpgradeMenu _ashud_main_menu true))
    (:NewEnumerator1
      (Default|StartCreditScore _ashud_main_menu))))

(event Collision|EventActorEndOverlap
  (params (OtherActor :type Actor%20Object%20Reference))
  (Utilities|Casting|CastToBP_Player OtherActor)
  (Rendering|Components|Sprite|SetSprite (Variables|Default|GetSprite) (Variables|Components|GetM%20NeutralSprite)))

(fn ConstructionScript
  (bind _m_neutralsprite (Variables|Components|GetM%20NeutralSprite))
  (Utilities|IsValid _m_neutralsprite
    (:Is%20Valid
      (Rendering|Components|Sprite|SetSprite (Variables|Default|GetSprite) _m_neutralsprite))))