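; Parent tower for a rat tower-defense game, initialized by type from templates with a list of shootable rat types.
; CheckNewRat, meant for child triggers, fills the focused-rat list, optionally single-target.
; Tick calls Shoot through a fire-rate Delay, damaging focused rats and spending limited shots before the tower destroys itself.
; Separate events stun or slow CC-flagged focused rats, or damage random rats from the game mode's spawn list (Mud).
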(event Custom|Shoot
  (bind _m_towertype (Variables|Components|GetM%20TowerType))
  ;[1 1 1] Shoot With DMG
  (for _array_element (Variables|Targets|GetM%20FocusedRats)
    ;;[1 1 1] Damages
    (bind _output_get (Variables|/Game/Blueprints/Actors/Enemy/BP_BaseRats.BP_BaseRats_C|SetratType _array_element (Utilities|Struct|MakeSTRUCT_Rat (.type (Variables|/Game/Blueprints/Actors/Enemy/BP_BaseRats.BP_BaseRats_C|GetratType _array_element)) (.isflying (Variables|/Game/Blueprints/Actors/Enemy/BP_BaseRats.BP_BaseRats_C|GetratType _array_element)) (.iscc (Variables|/Game/Blueprints/Actors/Enemy/BP_BaseRats.BP_BaseRats_C|GetratType _array_element)) (.element (Variables|/Game/Blueprints/Actors/Enemy/BP_BaseRats.BP_BaseRats_C|GetratType _array_element)) (- (.hp (Variables|/Game/Blueprints/Actors/Enemy/BP_BaseRats.BP_BaseRats_C|GetratType _array_element)) (.damage _m_towertype)) (.speed (Variables|/Game/Blueprints/Actors/Enemy/BP_BaseRats.BP_BaseRats_C|GetratType _array_element)) (.damage (Variables|/Game/Blueprints/Actors/Enemy/BP_BaseRats.BP_BaseRats_C|GetratType _array_element)))))
    (Development|PrintString (Utilities|String|Append "I SHOT MY TARGETS" " " (Utilities|String|ToString(Float) (.hp (Variables|/Game/Blueprints/Actors/Enemy/BP_BaseRats.BP_BaseRats_C|GetratType _array_element)))))
    (Utilities|FlowControl|Sequence
      (:then_0
        ;;[1 1 1] HP / NbShots
        (bind _result (Math|Integer|DecrementInt (.nbshots _m_towertype))
          (:%20%20
            (if (== _result 0)
              (Actor|DestroyActor)))))
      (:then_1
        (if (<= (.hp _output_get) 0.0)
          (CallFunction|RemoveRat _array_element)
          (Actor|DestroyActor))))))

(event Custom|Init
  (params (Tower%20type :type ENUM_Towers%20Enum :default "NewEnumerator0"))
  ;[1 1 1] Initializations : Tower type & shootable rats
  (bind _output_get (Variables|Components|SetM%20TowerType (Utilities|Array|Get(acopy) (.towers (Variables|Templates|GetM%20TowerTemplates)) (Math|Conversions|ToInteger(Byte) Tower%20type))))
  (bind _return (CallFunction|GetShootableRats (.type _output_get)))
  (Variables|Targets|SetM%20ShootableRats _return))

(event Custom|Stunt
  ;[1 1 1] Shoot with stun
  (for _array_element (Variables|Targets|GetM%20FocusedRats)
    ;;[1 1 1] Speed to 0
    (if (.iscc (Variables|/Game/Blueprints/Actors/Enemy/BP_BaseRats.BP_BaseRats_C|GetratType _array_element))
      (bind _output_get (Variables|/Game/Blueprints/Actors/Enemy/BP_BaseRats.BP_BaseRats_C|SetratType _array_element (Utilities|Struct|MakeSTRUCT_Rat (.type (Variables|/Game/Blueprints/Actors/Enemy/BP_BaseRats.BP_BaseRats_C|GetratType _array_element)) (.isflying (Variables|/Game/Blueprints/Actors/Enemy/BP_BaseRats.BP_BaseRats_C|GetratType _array_element)) (.iscc (Variables|/Game/Blueprints/Actors/Enemy/BP_BaseRats.BP_BaseRats_C|GetratType _array_element)) (.element (Variables|/Game/Blueprints/Actors/Enemy/BP_BaseRats.BP_BaseRats_C|GetratType _array_element)) (.hp (Variables|/Game/Blueprints/Actors/Enemy/BP_BaseRats.BP_BaseRats_C|GetratType _array_element)) 0.0 (.damage (Variables|/Game/Blueprints/Actors/Enemy/BP_BaseRats.BP_BaseRats_C|GetratType _array_element)))))
      ;;[1 1 1] Delay and speed reset
      (Utilities|FlowControl|Delay 0.5)
      (Variables|/Game/Blueprints/Actors/Enemy/BP_BaseRats.BP_BaseRats_C|SetratType _array_element (Utilities|Struct|MakeSTRUCT_Rat (.type _output_get) (.isflying _output_get) (.iscc _output_get) (.element _output_get) (.hp _output_get) (.speed (Variables|/Game/Blueprints/Actors/Enemy/BP_BaseRats.BP_BaseRats_C|GetratType _array_element)) (.damage _output_get)))
      (Utilities|FlowControl|Sequence
        (:then_0
          ;;[1 1 1] HP / NbShots
          (bind _result (Math|Integer|DecrementInt (.nbshots (Variables|Components|GetM%20TowerType)))
            (:%20%20
              (if (== _result 0)
                (Actor|DestroyActor)))))))))

(event Custom|Slow
  ;[1 1 1] Shoot with slow
  (for _array_element (Variables|Targets|GetM%20FocusedRats)
    ;;[1 1 1] Speed to / 2
    (if (.iscc (Variables|/Game/Blueprints/Actors/Enemy/BP_BaseRats.BP_BaseRats_C|GetratType _array_element))
      (bind _output_get (Variables|/Game/Blueprints/Actors/Enemy/BP_BaseRats.BP_BaseRats_C|SetratType _array_element (Utilities|Struct|MakeSTRUCT_Rat (.type (Variables|/Game/Blueprints/Actors/Enemy/BP_BaseRats.BP_BaseRats_C|GetratType _array_element)) (.isflying (Variables|/Game/Blueprints/Actors/Enemy/BP_BaseRats.BP_BaseRats_C|GetratType _array_element)) (.iscc (Variables|/Game/Blueprints/Actors/Enemy/BP_BaseRats.BP_BaseRats_C|GetratType _array_element)) (.element (Variables|/Game/Blueprints/Actors/Enemy/BP_BaseRats.BP_BaseRats_C|GetratType _array_element)) (.hp (Variables|/Game/Blueprints/Actors/Enemy/BP_BaseRats.BP_BaseRats_C|GetratType _array_element)) (.Remainder (Math|Float|Division(WholeandRemainder) (.speed (Variables|/Game/Blueprints/Actors/Enemy/BP_BaseRats.BP_BaseRats_C|GetratType _array_element)) 2.0)) (.damage (Variables|/Game/Blueprints/Actors/Enemy/BP_BaseRats.BP_BaseRats_C|GetratType _array_element)))))
      ;;[1 1 1] Delay and speed reset
      (Utilities|FlowControl|Delay 0.5)
      (Variables|/Game/Blueprints/Actors/Enemy/BP_BaseRats.BP_BaseRats_C|SetratType _array_element (Utilities|Struct|MakeSTRUCT_Rat (.type _output_get) (.isflying _output_get) (.iscc _output_get) (.element _output_get) (.hp _output_get) (.speed (Variables|/Game/Blueprints/Actors/Enemy/BP_BaseRats.BP_BaseRats_C|GetratType _array_element)) (.damage _output_get)))
      (Utilities|FlowControl|Sequence
        (:then_0
          ;;[1 1 1] HP / NbShots
          (bind _result (Math|Integer|DecrementInt (.nbshots (Variables|Components|GetM%20TowerType)))
            (:%20%20
              (if (== _result 0)
                (Actor|DestroyActor)))))))))

(event Custom|Mud
  ;[1 1 1] Mud
  (bind _asgm_play_mode (Utilities|Casting|CastToGM_PlayMode (Game|GetGameMode)))
  (if (not (== (Utilities|Array|Length (Variables|/Game/Blueprints/Gamemodes/GM_PlayMode.GM_PlayMode_C|GetM%20SpawnedRats _asgm_play_mode)) 0))
    (bind _output_get (Variables|/Game/Blueprints/Actors/Enemy/BP_BaseRats.BP_BaseRats_C|SetratType (Utilities|Array|Get(acopy) (Variables|/Game/Blueprints/Gamemodes/GM_PlayMode.GM_PlayMode_C|GetM%20SpawnedRats _asgm_play_mode) (Math|Random|RandomIntegerinRange 0 (- (Utilities|Array|Length (Variables|/Game/Blueprints/Gamemodes/GM_PlayMode.GM_PlayMode_C|GetM%20SpawnedRats _asgm_play_mode)) 1))) (Utilities|Struct|MakeSTRUCT_Rat (.type (Variables|/Game/Blueprints/Actors/Enemy/BP_BaseRats.BP_BaseRats_C|GetratType (Utilities|Array|Get(acopy) (Variables|/Game/Blueprints/Gamemodes/GM_PlayMode.GM_PlayMode_C|GetM%20SpawnedRats _asgm_play_mode) (Math|Random|RandomIntegerinRange 0 (- (Utilities|Array|Length (Variables|/Game/Blueprints/Gamemodes/GM_PlayMode.GM_PlayMode_C|GetM%20SpawnedRats _asgm_play_mode)) 1))))) (.isflying (Variables|/Game/Blueprints/Actors/Enemy/BP_BaseRats.BP_BaseRats_C|GetratType (Utilities|Array|Get(acopy) (Variables|/Game/Blueprints/Gamemodes/GM_PlayMode.GM_PlayMode_C|GetM%20SpawnedRats _asgm_play_mode) (Math|Random|RandomIntegerinRange 0 (- (Utilities|Array|Length (Variables|/Game/Blueprints/Gamemodes/GM_PlayMode.GM_PlayMode_C|GetM%20SpawnedRats _asgm_play_mode)) 1))))) (.iscc (Variables|/Game/Blueprints/Actors/Enemy/BP_BaseRats.BP_BaseRats_C|GetratType (Utilities|Array|Get(acopy) (Variables|/Game/Blueprints/Gamemodes/GM_PlayMode.GM_PlayMode_C|GetM%20SpawnedRats _asgm_play_mode) (Math|Random|RandomIntegerinRange 0 (- (Utilities|Array|Length (Variables|/Game/Blueprints/Gamemodes/GM_PlayMode.GM_PlayMode_C|GetM%20SpawnedRats _asgm_play_mode)) 1))))) (.element (Variables|/Game/Blueprints/Actors/Enemy/BP_BaseRats.BP_BaseRats_C|GetratType (Utilities|Array|Get(acopy) (Variables|/Game/Blueprints/Gamemodes/GM_PlayMode.GM_PlayMode_C|GetM%20SpawnedRats _asgm_play_mode) (Math|Random|RandomIntegerinRange 0 (- (Utilities|Array|Length (Variables|/Game/Blueprints/Gamemodes/GM_PlayMode.GM_PlayMode_C|GetM%20SpawnedRats _asgm_play_mode)) 1))))) (- (.hp (Variables|/Game/Blueprints/Actors/Enemy/BP_BaseRats.BP_BaseRats_C|GetratType (Utilities|Array|Get(acopy) (Variables|/Game/Blueprints/Gamemodes/GM_PlayMode.GM_PlayMode_C|GetM%20SpawnedRats _asgm_play_mode) (Math|Random|RandomIntegerinRange 0 (- (Utilities|Array|Length (Variables|/Game/Blueprints/Gamemodes/GM_PlayMode.GM_PlayMode_C|GetM%20SpawnedRats _asgm_play_mode)) 1))))) 1e+02) (.speed (Variables|/Game/Blueprints/Actors/Enemy/BP_BaseRats.BP_BaseRats_C|GetratType (Utilities|Array|Get(acopy) (Variables|/Game/Blueprints/Gamemodes/GM_PlayMode.GM_PlayMode_C|GetM%20SpawnedRats _asgm_play_mode) (Math|Random|RandomIntegerinRange 0 (- (Utilities|Array|Length (Variables|/Game/Blueprints/Gamemodes/GM_PlayMode.GM_PlayMode_C|GetM%20SpawnedRats _asgm_play_mode)) 1))))) (.damage (Variables|/Game/Blueprints/Actors/Enemy/BP_BaseRats.BP_BaseRats_C|GetratType (Utilities|Array|Get(acopy) (Variables|/Game/Blueprints/Gamemodes/GM_PlayMode.GM_PlayMode_C|GetM%20SpawnedRats _asgm_play_mode) (Math|Random|RandomIntegerinRange 0 (- (Utilities|Array|Length (Variables|/Game/Blueprints/Gamemodes/GM_PlayMode.GM_PlayMode_C|GetM%20SpawnedRats _asgm_play_mode)) 1))))))))
    (if (<= (.hp _output_get) 0.0)
      (Actor|DestroyActor (Utilities|Array|Get(acopy) (Variables|/Game/Blueprints/Gamemodes/GM_PlayMode.GM_PlayMode_C|GetM%20SpawnedRats _asgm_play_mode) (Math|Random|RandomIntegerinRange 0 (- (Utilities|Array|Length (Variables|/Game/Blueprints/Gamemodes/GM_PlayMode.GM_PlayMode_C|GetM%20SpawnedRats _asgm_play_mode)) 1)))))))

(event Custom|CheckNewRat
  (params (RatRef :type BP%20Base%20Rats%20Object%20Reference))
  ;[1 1 1 1 50] Handles focused rats
  ;;[1 1 1] May be called by child (Depends on the trigger type
  (if (Variables|Targets|GetM%20SingleTarget)
    (if (== (Utilities|Array|Length (Variables|Targets|GetM%20FocusedRats)) 0)
      (bind _return (CallFunction|IsRatShootable (Variables|/Game/Blueprints/Actors/Enemy/BP_BaseRats.BP_BaseRats_C|GetratType RatRef) :!label _label))
      (if _return
        (Utilities|Array|Add (Variables|Targets|GetM%20FocusedRats) RatRef)))
    (else
      (goto _label))))

(event Custom|RemoveRat
  (params (Rat%20ref :type BP%20Base%20Rats%20Object%20Reference))
  ;[1 1 1 1 50] Handles focused rats
  (Utilities|Array|RemoveItem (Variables|Targets|GetM%20FocusedRats) Rat%20ref))

(event EventTick
  (params (DeltaSeconds :type Float%20%28single-precision%29))
  ;[1 1 1] Calls Shooting
  (Utilities|FlowControl|Delay (.firerate (Variables|Components|GetM%20TowerType)))
  (CallFunction|Shoot))

(fn ConstructionScript)

(fn GetShootableRats
  (params (Tower%20type :type ENUM_Towers%20Enum :default "NewEnumerator0"))
  (bind _fillingshootables (LocalVariables|GetFillingShootables))
  (for _array_element (.rats (Variables|Templates|GetM%20RatTemplates))
    (switch Utilities|FlowControl|Switch|SwitchonENUM_Towers Tower%20type
      (:NewEnumerator0
        (if (not (.IsFlying (Utilities|Struct|BreakSTRUCT_Rat _array_element))) :!label _label
          (if (Utilities|Enum|NotEqual(Enum) (.Type (Utilities|Struct|BreakSTRUCT_Rat _array_element)) "NewEnumerator4") :!label _label_2
            (Utilities|Array|Add _fillingshootables _array_element))))
      (:NewEnumerator1
        (goto _label_2))
      (:NewEnumerator2
        (if (not (.IsCC (Utilities|Struct|BreakSTRUCT_Rat _array_element)))
          (goto _label_2)))
      (:NewEnumerator3
        (goto _label_2))
      (:NewEnumerator4
        (if (and (not (.IsFlying (Utilities|Struct|BreakSTRUCT_Rat _array_element))) (not (.IsCC (Utilities|Struct|BreakSTRUCT_Rat _array_element))))
          (goto _label_2)))
      (:NewEnumerator5
        (goto _label_2))
      (:NewEnumerator6
        (goto _label))
      (:NewEnumerator7
        (goto _label))
      (:NewEnumerator8
        (goto _label_2))
      (:NewEnumerator9
        (goto _label))))
  (return _fillingshootables))

(fn CanShoot
  (params (Rat :type STRUCT%20Rat%20Structure))
  (return false))

(fn IsRatShootable
  (params (Rat :type STRUCT%20Rat%20Structure))
  (for _array_element (Variables|Targets|GetM%20ShootableRats)
    (if (Utilities|RatStructEqual _array_element Rat)
      (return true)))
  (return false))