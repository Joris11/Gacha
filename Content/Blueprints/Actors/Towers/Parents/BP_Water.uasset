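; BP_Water is a water tower Blueprint that slows rats entering its range.
; It plays an intro sound at the mesh location on BeginPlay.
; Sphere overlaps add each BP_BaseRats to the focused-rat list and call Slow, then call RemoveRat when one leaves.
; Slow and RemoveRat are called here but defined outside these graphs.
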(event OnComponentBeginOverlap(Sphere)
  (params (OverlappedComponent :type Primitive%20Component%20Object%20Reference) (OtherActor :type Actor%20Object%20Reference) (OtherComp :type Primitive%20Component%20Object%20Reference) (OtherBodyIndex :type Integer) (bFromSweep :type Boolean) (SweepResult :type Hit%20Result%20Structure%20%28by%20ref%29))
  (bind _asbp_base_rats (Utilities|Casting|CastToBP_BaseRats OtherActor))
  (Utilities|Array|Add (Variables|Default|GetM%20FocusedRats) _asbp_base_rats)
  (CallFunction|Slow))

(event OnComponentEndOverlap(Sphere)
  (params (OverlappedComponent :type Primitive%20Component%20Object%20Reference) (OtherActor :type Actor%20Object%20Reference) (OtherComp :type Primitive%20Component%20Object%20Reference) (OtherBodyIndex :type Integer))
  (bind _asbp_base_rats (Utilities|Casting|CastToBP_BaseRats OtherActor))
  (CallFunction|RemoveRat _asbp_base_rats))

(event EventBeginPlay
  (Audio|PlaySoundatLocation "/Game/Sounds/Tower_sounds/Tower-Water-Intro.Tower-Water-Intro" (Transformation|GetWorldLocation (Variables|Character|GetMesh))))

(event Collision|EventActorBeginOverlap
  (params (OtherActor :type Actor%20Object%20Reference)))

(event EventTick
  (params (DeltaSeconds :type Float%20%28single-precision%29)))

(fn ConstructionScript)