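; BP_ConeTower is a tower Blueprint that detects rats with a box range trigger, apparently as a parent for cone-range towers.
; Construction runs the parent script, then sets the box's Y extent from the tower type's Range.
; Overlapping BP_BaseRats actors go to CheckNewRat if the tower type has range, and RemoveRat handles them when they leave.
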(event OnComponentEndOverlap(RangeTrigger)
  (params (OverlappedComponent :type Primitive%20Component%20Object%20Reference) (OtherActor :type Actor%20Object%20Reference) (OtherComp :type Primitive%20Component%20Object%20Reference) (OtherBodyIndex :type Integer))
  (bind _asbp_base_rats (Utilities|Casting|CastToBP_BaseRats OtherActor))
  (CallFunction|RemoveRat _asbp_base_rats))

(event OnComponentBeginOverlap(RangeTrigger)
  (params (OverlappedComponent :type Primitive%20Component%20Object%20Reference) (OtherActor :type Actor%20Object%20Reference) (OtherComp :type Primitive%20Component%20Object%20Reference) (OtherBodyIndex :type Integer) (bFromSweep :type Boolean) (SweepResult :type Hit%20Result%20Structure%20%28by%20ref%29))
  (bind _asbp_base_rats (Utilities|Casting|CastToBP_BaseRats OtherActor))
  (if (.hasrange (Variables|Default|GetM%20TowerType))
    (CallFunction|CheckNewRat _asbp_base_rats)))

(fn ConstructionScript
  (bind _rangetrigger (Variables|Default|GetRangeTrigger))
  (bind _boxextent (Variables|/Script/Engine.BoxComponent|GetBoxExtent _rangetrigger))
  (|CallParentFunction)
  (Components|Box|SetBoxExtent _rangetrigger (Math|Vector|MakeVector (.x _boxextent) (.range (Variables|Default|GetM%20TowerType)) (.z _boxextent)) true))