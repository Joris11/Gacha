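; BP_SphereTower is a parent tower Blueprint that detects rats within a spherical range.
; The construction script runs its parent's logic, then sizes the RangeTrigger sphere from the Range value in MTowerType.
; Overlapping BP_BaseRats actors go to CheckNewRat on entry if the tower type has range, and to RemoveRat on exit regardless of that flag.
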(event OnComponentBeginOverlap(RangeTrigger)
  (params (OverlappedComponent :type Primitive%20Component%20Object%20Reference) (OtherActor :type Actor%20Object%20Reference) (OtherComp :type Primitive%20Component%20Object%20Reference) (OtherBodyIndex :type Integer) (bFromSweep :type Boolean) (SweepResult :type Hit%20Result%20Structure%20%28by%20ref%29))
  (bind _asbp_base_rats (Utilities|Casting|CastToBP_BaseRats OtherActor))
  (if (.hasrange (Variables|Default|GetM%20TowerType))
    (CallFunction|CheckNewRat _asbp_base_rats)))

(event OnComponentEndOverlap(RangeTrigger)
  (params (OverlappedComponent :type Primitive%20Component%20Object%20Reference) (OtherActor :type Actor%20Object%20Reference) (OtherComp :type Primitive%20Component%20Object%20Reference) (OtherBodyIndex :type Integer))
  (bind _asbp_base_rats (Utilities|Casting|CastToBP_BaseRats OtherActor))
  (CallFunction|RemoveRat _asbp_base_rats))

(fn ConstructionScript
  (|CallParentFunction)
  (Components|Sphere|SetSphereRadius (Variables|Default|GetRangeTrigger) (.range (Variables|Default|GetM%20TowerType)) true))