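; BP_TowerRangeCone is a tower Blueprint that tracks rats within shooting range through a box trigger, ShotTrigger.
; The construction script sizes the box from MShotRange.
; Overlapping BP_BaseRats actors join MTargets only while it holds fewer than MMaxTargetPerShot, and leave it on end overlap.
; Rats entering when the list is full are not added later if a slot frees up.
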(event OnComponentBeginOverlap(ShotTrigger)
  (params (OverlappedComponent :type Primitive%20Component%20Object%20Reference) (OtherActor :type Actor%20Object%20Reference) (OtherComp :type Primitive%20Component%20Object%20Reference) (OtherBodyIndex :type Integer) (bFromSweep :type Boolean) (SweepResult :type Hit%20Result%20Structure%20%28by%20ref%29))
  ;[1 1 1] Add rats in range
  (bind _asbp_base_rats (Utilities|Casting|CastToBP_BaseRats OtherActor))
  (bind _return (CallFunction|CanAddTarget))
  (if _return
    (Utilities|Array|Add (Variables|Default|GetM%20Targets) _asbp_base_rats)))

(event OnComponentEndOverlap(ShotTrigger)
  (params (OverlappedComponent :type Primitive%20Component%20Object%20Reference) (OtherActor :type Actor%20Object%20Reference) (OtherComp :type Primitive%20Component%20Object%20Reference) (OtherBodyIndex :type Integer))
  ;[1 1 1] Add rats in range
  (bind _asbp_base_rats (Utilities|Casting|CastToBP_BaseRats OtherActor))
  (Utilities|Array|RemoveItem (Variables|Default|GetM%20Targets) _asbp_base_rats))

(event EventTick
  (params (DeltaSeconds :type Float%20%28single-precision%29))
  (|CallParentFunction DeltaSeconds) ; This node is disabled and will not be called.\nDrag off pins to build functionality.
)

(fn ConstructionScript
  (|CallParentFunction)
  (Components|Box|SetBoxExtent (Variables|Default|GetShotTrigger) (Variables|Components|GetM%20ShotRange) true))

(fn CanAddTarget
  (return (< (Utilities|Array|Length (Variables|Default|GetM%20Targets)) (Variables|Default|GetM%20MaxTargetPerShot))))