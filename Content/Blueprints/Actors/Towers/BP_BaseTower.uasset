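; Base tower actor that periodically shoots at rat targets, with ShootIt left empty, apparently for child towers to implement.
; Tick runs through a fire-rate Delay into TryShoot, which calls ShootIt on every target when targets exist and CheckOP passes.
; CheckOP sets the operational flag from whether the max shot count is above zero.
; Helpers clear that flag and report free target slots; target acquisition happens outside this graph.
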(event Custom|TryShoot
  (bind _return (CallFunction|CanShoot))
  (if _return
    (CallFunction|ShootEach)))

(event Custom|ShootEach
  (for _array_element (Variables|Components|GetM%20Targets)
    (CallFunction|ShootIt _array_element)))

(event Custom|ShootIt
  (params (RatToShoot :type BP%20Base%20Rats%20Object%20Reference)))

(event EventTick
  (params (DeltaSeconds :type Float%20%28single-precision%29))
  (Utilities|FlowControl|Delay (Variables|Components|GetM%20FireRate))
  (CallFunction|TryShoot))

(fn ConstructionScript)

(fn DisableTower
  (Variables|Components|SetM%20IsOP false))

(fn CheckOP
  (bind _output_get (Variables|Components|SetM%20IsOP (> (Variables|Components|GetM%20MaxNbShots) 0)))
  (return _output_get))

(fn CanShoot
  (bind _return (CallFunction|CheckOP))
  (return (and (> (Utilities|Array|Length (Variables|Components|GetM%20Targets)) 0) _return)))

(fn HasTargetsSpace
  (return (< (Utilities|Array|Length (Variables|Components|GetM%20Targets)) (Variables|Components|GetM%20MaxTargetPerShot))))